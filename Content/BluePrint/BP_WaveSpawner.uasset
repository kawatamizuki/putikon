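; BP_WaveSpawner is an actor that spawns enemies in sequential waves, starting at BeginPlay.
; Each Waves entry sets enemy class, count, spawn interval and post-wave delay, and enemies spawn one by one at the spawner's transform, receiving its PathActor.
; It then polls every second until no actors of that class remain, waits, and advances to the next wave, stopping when the index runs past the array.
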(event `CheckWaveClear`
  (bind _outactors (`GameplayStatics.GetAllActorsOfClass` (`self.EnemyClass`)))
  (if (== (`KismetArrayLibrary.Array_Length` _outactors) 0)
    (`KismetSystemLibrary.Delay` (`self.DelayAfterWave`))
    (`/Engine/EditorBlueprintResources/StandardMacros.IncrementInt` (`self.CurrentWaveIndex`)
      (:`  `
        (`self.StartCurrentWave` :!label _label)))
    (else
      (`KismetSystemLibrary.Delay` 1.0)
      (`self.CheckWaveClear`))))

(event `self.ReceiveBeginPlay`
  (goto _label))

(event `SpawnNextEnemy`
  (if (< (`self.SpawnedCount`) (`self.EnemyCount`))
    (`|SpawnActorFromClass` (`self.EnemyClass`) (`self.GetTransform`) "AlwaysSpawn" "MultiplyWithRoot" null (`self.PathActor`) null)
    (`/Engine/EditorBlueprintResources/StandardMacros.IncrementInt` (`self.SpawnedCount`)
      (:`  `
        (`KismetSystemLibrary.Delay` (`self.SpawnInterval`))
        (`self.SpawnNextEnemy`)))
    (else
      (`self.CheckWaveClear`))))

(event `StartCurrentWave`
  (bind (_output_enemyclass _output_enemycount _output_spawninterval _output_delayafterwave) (break `/Game/BluePrint/ST_WaveData` (`|GetArrayItem` (`self.Waves`) (`self.CurrentWaveIndex`))))
  (if (`KismetArrayLibrary.Array_IsValidIndex` (`self.Waves`) (`self.CurrentWaveIndex`))
    (set `self.EnemyClass` _output_enemyclass)
    (set `self.EnemyCount` _output_enemycount)
    (set `self.SpawnInterval` _output_spawninterval)
    (set `self.DelayAfterWave` _output_delayafterwave)
    (set `self.SpawnedCount` 0)
    (`self.SpawnNextEnemy`)))

(fn `UserConstructionScript`)