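; BP_BuildTree is a tree that serves as a tower build spot, highlighted when the player character is nearby.
; Its BuildRange overlap sets or clears the character's CurrentBuildTree and starts or stops a highlight timeline, resetting Pulse on exit.
; The highlight uses a dynamic material instance as the mesh's overlay material, with the timeline meant to drive its Pulse parameter.
; OnTowerBuilt plays the tower placement sound at the tree's location.
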(event `self.ReceiveBeginPlay`
  (bind _returnvalue (`KismetMaterialLibrary.CreateDynamicMaterialInstance` "/Game/Materials/M_TreeHighlight.M_TreeHighlight"))
  (bind _output_get (set `self.HighlightMID` _returnvalue))
  (`MeshComponent.SetOverlayMaterial` (`self.TreeMesh`) _output_get))

(event `self.BuildRange.OnComponentBeginOverlap`
  (params (OverlappedComponent :type "PrimitiveComponent Object Reference") (OtherActor :type "Actor Object Reference") (OtherComp :type "PrimitiveComponent Object Reference") (OtherBodyIndex :type Integer) (bFromSweep :type Boolean) (SweepResult :type "HitResult Structure (by ref)"))
  (bind _asbp_third_person_character (cast `/Game/ThirdPerson/Blueprints/BP_ThirdPersonCharacter` OtherActor))
  (set `/Game/ThirdPerson/Blueprints/BP_ThirdPersonCharacter.CurrentBuildTree` self _asbp_third_person_character)
  (`TimelineComponent.PlayFromStart` (`self.TL_HighlightPulse`)))

(event `self.BuildRange.OnComponentEndOverlap`
  (params (OverlappedComponent :type "PrimitiveComponent Object Reference") (OtherActor :type "Actor Object Reference") (OtherComp :type "PrimitiveComponent Object Reference") (OtherBodyIndex :type Integer))
  (bind _asbp_third_person_character (cast `/Game/ThirdPerson/Blueprints/BP_ThirdPersonCharacter` OtherActor))
  (set `/Game/ThirdPerson/Blueprints/BP_ThirdPersonCharacter.CurrentBuildTree` null _asbp_third_person_character)
  (`TimelineComponent.Stop` (`self.TL_HighlightPulse`))
  (`MaterialInstanceDynamic.SetScalarParameterValue` (`self.HighlightMID`) "Pulse" 0.0))

(event `self.OnTowerBuilt`
  (`GameplayStatics.PlaySoundAtLocation` "/Game/Sounds/タワー設置音.タワー設置音" (`self.K2_GetActorLocation`) (struct) 2.0 1.0 0.0 null null null null))

(fn `UserConstructionScript`)